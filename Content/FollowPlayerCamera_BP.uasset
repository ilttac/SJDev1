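; FollowPlayerCamera_BP is an actor, named as a camera, that follows the player along the world Y axis.
; On BeginPlay it finds and caches the MyCSJPlayer actor with GetActorOfClass.
; Every Tick it copies that player's Y location to itself, keeping its own X, Z and rotation and setting scale to one, with no smoothing or validity check.
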(event EventBeginPlay
  (bind _returnvalue (Actor|GetActorOfClass "/Game/SJCharacter/MyCSJPlayer.MyCSJPlayer_C")))

(event Collision|EventActorBeginOverlap
  (params (OtherActor :type Actor%20Object%20Reference)))

(event EventTick
  (params (DeltaSeconds :type Float%20%28single-precision%29))
  (bind _returnvalue (Transformation|GetActorLocation))
  (bind (_x _y _z) (Math|Vector|BreakVector _returnvalue))
  (if true
    (Transformation|SetActorTransform (Math|Transform|MakeTransform (Math|Vector|MakeVector _x (.Y (Math|Vector|BreakVector (Transformation|GetActorLocation (stale EventBeginPlay _returnvalue)))) _z) (Transformation|GetActorRotation)))))

(fn ConstructionScript)